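; Main menu ambience manager that plays random sounds and periodic light blackouts when the game state is MainMenu.
; Five seconds after BeginPlay it gathers level Light actors, plus light components and dynamic mesh materials from BP_LSMap actors.
; Two self-rescheduling random-delay loops drive it.
; LoopLight plays a cue, briefly hides lights and zeroes emissive; LoopSound plays one of three cues, some repeated.
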(event `self.ReceiveBeginPlay`
  (`KismetSystemLibrary.Delay` 5.0)
  ; MainMenu일 시 소리 재생 및 lighting 효과
  (bind _aspggame_state (cast `PGGameState` (`GameplayStatics.GetGameState`)))
  (`/Engine/EditorBlueprintResources/StandardMacros.IsValid` _aspggame_state
    (:`Is Valid`
      (if (`|EnumEquality` (`PGGameState.CurrentGameState` _aspggame_state) "MainMenu")
        (`KismetSystemLibrary.PrintString` "MainMenuTrue" false true (struct :`G` 0.66 :`B` 1.0 :`A` 1.0) 0.1)
        (`|ExecutionSequence`
          (:`then_0`
            (`self.LoopLight`)
            (`|ExecutionSequence`
              (:`then_0`
                (bind _outactors (`GameplayStatics.GetAllActorsOfClass` "/Game/ProjectG/Levels/LevelSequence/BP_LSMap.BP_LSMap_C"))
                (for _array_element _outactors
                  (set `self.LightComponents` (`self.K2_GetComponentsByClass` _array_element "/Script/Engine.LightComponent"))))
              (:`then_1`
                (for _array_element_2 _outactors
                  (for _array_element_3 (`self.K2_GetComponentsByClass` _array_element_2 "/Script/Engine.StaticMeshComponent")
                    (bind _returnvalue (`PrimitiveComponent.CreateDynamicMaterialInstance` _array_element_3 0 null "None"))
                    (`KismetArrayLibrary.Array_Add` (`self.LightMIDs`) _returnvalue))))
              (:`then_2`
                (bind _outactors_2 (`GameplayStatics.GetAllActorsOfClass` "/Script/Engine.Light"))
                (bind _output_get (set `self.Lights` _outactors_2))
                (for _ _output_get
                  _))))
          (:`then_1`
            (`self.LoopSound`)))))))

(event `LoopSound`
  (bind _audio (`self.Audio`))
  (bind _soundcues (`self.SoundCues`))
  (`KismetSystemLibrary.Delay` (`KismetMathLibrary.RandomFloatInRange` 15.0 25.0))
  (`|ExecutionSequence`
    (:`then_0`
      (`self.LoopSound`))
    (:`then_1`
      (switch `int` (`KismetMathLibrary.RandomIntegerInRange` 0 2)
        (:`0`
          (`AudioComponent.SetSound` _audio (`|GetArrayItem` _soundcues))
          (`AudioComponent.Play` _audio 0.0))
        (:`1`
          (`AudioComponent.SetSound` _audio (`|GetArrayItem` _soundcues 1))
          (`AudioComponent.Play` _audio 0.0)
          (`KismetSystemLibrary.Delay` 3.0)
          (`AudioComponent.Play` _audio 0.0))
        (:`2`
          (`AudioComponent.SetSound` _audio (`|GetArrayItem` _soundcues 2))
          (`AudioComponent.Play` _audio 0.0)
          (`KismetSystemLibrary.Delay` 1.3)
          (`AudioComponent.Play` _audio 0.0)
          (`KismetSystemLibrary.Delay` 1.3)
          (`AudioComponent.Play` _audio 0.0))))))

(event `LoopLight`
  (`KismetSystemLibrary.Delay` (`KismetMathLibrary.RandomFloatInRange` 7.0 10.0))
  (`GameplayStatics.PlaySound2D` "/Game/Imports/Sounds/Levels/Environment/SC_MainMenuLightOut.SC_MainMenuLightOut" 1.0 1.0 0.0 null null)
  (`|ExecutionSequence`
    (:`then_0`
      (`self.LoopLight`))
    (:`then_1`
      (for _array_element (`self.Lights`)
        (bind _lightcomponent (`Light.LightComponent` _array_element))
        (`/Engine/EditorBlueprintResources/StandardMacros.IsValid` _lightcomponent
          (:`Is Valid`
            (`SceneComponent.SetVisibility` _lightcomponent false false))))
      (`KismetSystemLibrary.Delay` 0.5)
      (for _array_element_2 (`self.Lights`)
        (bind _lightcomponent_2 (`Light.LightComponent` _array_element_2))
        (`/Engine/EditorBlueprintResources/StandardMacros.IsValid` _lightcomponent_2
          (:`Is Valid`
            (`SceneComponent.SetVisibility` _lightcomponent_2 true false)))))
    (:`then_2`
      (for _array_element_3 (`self.LightComponents`)
        ; Light Components(전구 밝기)
        (`/Engine/EditorBlueprintResources/StandardMacros.IsValid` _array_element_3
          (:`Is Valid`
            (`SceneComponent.SetVisibility` _array_element_3 false false))))
      (`KismetSystemLibrary.Delay` 0.5)
      (for _array_element_4 (`self.LightComponents`)
        (`/Engine/EditorBlueprintResources/StandardMacros.IsValid` _array_element_4
          (:`Is Valid`
            (`SceneComponent.SetVisibility` _array_element_4 true false)))))
    (:`then_3`
      (for _array_element_5 (`self.LightMIDs`)
        (`/Engine/EditorBlueprintResources/StandardMacros.IsValid` _array_element_5
          (:`Is Valid`
            (`MaterialInstanceDynamic.SetScalarParameterValue` _array_element_5 "EmissiveValue" 0.0))))
      (`KismetSystemLibrary.Delay` 0.5)
      (for _array_element_6 (`self.LightMIDs`)
        (`/Engine/EditorBlueprintResources/StandardMacros.IsValid` _array_element_6
          (:`Is Valid`
            (`MaterialInstanceDynamic.SetScalarParameterValue` _array_element_6 "EmissiveValue" 8.0)))))))

(fn `UserConstructionScript`)