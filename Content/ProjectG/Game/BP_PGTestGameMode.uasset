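; BP_PGTestGameMode is a test game mode that spawns a ground piece and a monster and builds the navmesh, once, after a short startup delay.
; Tick accumulates a timer, and a boolean latch limits the trigger to a single firing.
; It casts the current game mode to its own class and calls TESTMakeGroundSpawnMonsterAndBuildNavMesh with hardcoded spawn locations and ground scale.
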(event `self.ReceiveBeginPlay`)

(event `self.ReceiveTick`
  (params (DeltaSeconds :type "Float (single-precision)"))
  (set `self.SpawnTimer` (+ (`self.SpawnTimer`) DeltaSeconds))
  (if (> (`self.SpawnTimer`) 2.0)
    (if (not (`self.TriggerOnlyOnce`))
      (bind _asbp_pgtest_game_mode (cast `/Game/ProjectG/Game/BP_PGTestGameMode` (`GameplayStatics.GetGameMode`)))
      (`self.TEST_MakeGroundSpawnMonsterAndBuildNavMesh` _asbp_pgtest_game_mode (1350.0 2620.0 110.0) (1360.0 2570.0 -40.0) (6.0 6.5 1.0))
      (set `self.TriggerOnlyOnce` true))))

(fn `UserConstructionScript`)