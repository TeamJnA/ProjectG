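; Game instance blueprint for Advanced Sessions multiplayer in ProjectG, currently inert because none of its session logic is connected to an event.
; The CreateSession and OnSessionInviteAccepted events are empty.
; Orphaned chains would create a session and open the lobby as a listen server, find and join the first session, or join an invite's session.
; The create and invite chains first destroy any existing session, continuing even if that fails.
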(event `CreateSession`)

(event `self.OnSessionInviteAccepted`
  (params (LocalPlayerNum :type Integer) (PersonInvited :type "BPUniqueNetId Structure") (SessionToJoin :type "BlueprintSessionResult Structure (by ref)")))