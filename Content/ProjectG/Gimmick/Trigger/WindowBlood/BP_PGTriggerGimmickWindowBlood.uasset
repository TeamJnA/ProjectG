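; BP_PGTriggerGimmickWindowBlood is a trigger gimmick Blueprint, apparently for a blood-on-window effect.
; On BeginPlay it gathers its individual BloodEffect references into EffectArray in a hand-picked, non-numeric order.
; The graph has no trigger or playback logic of its own; the overlap and tick events are disabled and the construction script is empty.
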(event `self.ReceiveBeginPlay`
  (set `self.EffectArray` (`|MakeArray` (`self.BloodEffect16`) (`self.BloodEffect4`) (`self.BloodEffect3`) (`self.BloodEffect2`) (`self.BloodEffect6`) (`self.BloodEffect1`) (`self.BloodEffect0`) (`self.BloodEffect7`) (`self.BloodEffect17`) (`self.BloodEffect5`) (`self.BloodEffect15`) (`self.BloodEffect14`) (`self.BloodEffect12`) (`self.BloodEffect13`) (`self.BloodEffect11`) (`self.BloodEffect10`) (`self.BloodEffect9`) (`self.BloodEffect8`))))

(fn `UserConstructionScript`)